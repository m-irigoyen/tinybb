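; Player controller for TinyBB, a tabletop-style game with team minis and a ball, linked to a TinyBBHUD widget.
; Clicking selects a mini, dragging moves it via cursor trace with an authority-only location update, and release snaps it to grid.
; Input actions spawn or delete minis and toggle ball, done, prone and stunned states, then refresh renderers.
; Save and init-file loading are unfinished: quicksave writes an empty string.
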(event Custom|SetMiniLocation
  (params (mini :type Actor%20Object%20Reference) (location :type Vector))
  (Networking|SwitchHasAuthority
    (:Authority
      (Transformation|SetActorLocation mini location false false))))

(event Custom|Update%20Mini%20Renderers
  (params (mini :type Mini%20Object%20Reference))
  (Default|UpdateRenderers mini))

(event Custom|SnapMiniToGrid
  (params (mini :type Mini%20Object%20Reference))
  (Default|SnaptoGrid mini))

(event Custom|MiniToggleProne
  (params (mini :type Mini%20Object%20Reference))
  (Default|ToggleProne mini)
  (CallFunction|UpdateMiniRenderers mini))

(event Custom|MiniToggleStunned
  (params (mini :type Mini%20Object%20Reference))
  (Default|ToggleStunned mini)
  (CallFunction|UpdateMiniRenderers mini))

(event Custom|MiniToggleBall
  (params (mini :type Mini%20Object%20Reference))
  (Default|ToggleBall mini)
  (CallFunction|UpdateMiniRenderers mini))

(event Custom|MiniToggleDone
  (params (mini :type Mini%20Object%20Reference))
  (Default|ToggleDone mini)
  (CallFunction|UpdateMiniRenderers mini))

(event EventTick
  (params (DeltaSeconds :type Float%20%28single-precision%29))
  (bind (_worldlocation _worlddirection) (Game|Player|ConvertMouseLocationToWorldSpace))
  (if (and (Utilities|IsValid (Variables|Default|GetselectedMini)) (Variables|Default|Getclicking))
    (bind _outhit (Collision|LineTraceForObjects _worldlocation (+ _worldlocation (* _worlddirection 1e+05)) (Utilities|Array|MakeArray "ObjectTypeQuery1") false 0 "None"))
    (CallFunction|SetMiniLocation (Variables|Default|GetselectedMini) (Math|Vector|MakeVector (.X (Math|Vector|BreakVector (.Location (Collision|BreakHitResult _outhit)))) (.Y (Math|Vector|BreakVector (.Location (Collision|BreakHitResult _outhit)))) 0.0))))

(event EventBeginPlay
  (bind _returnvalue (UserInterface|CreateWidget "/Game/Blueprints/TinyBBHUD.TinyBBHUD_C"))
  (UserInterface|Viewport|AddtoViewport _returnvalue 0)
  (Variables|/Game/Blueprints/TinyBBHUD.TinyBBHUD_C|SettinyBBcontroller _returnvalue self)
  (Variables|Default|SethudRef _returnvalue))

(event Input|ActionEvents|InputActionToggleBall
  (params (Key :type Key%20Structure :default "AnyKey"))
  (bind _selectedmini (Variables|Default|GetselectedMini))
  (:Pressed
    (if (Utilities|IsValid _selectedmini)
      (CallFunction|MiniToggleBall _selectedmini))))

(event Input|ActionEvents|InputActionToggleProne
  (params (Key :type Key%20Structure :default "AnyKey"))
  (bind _selectedmini (Variables|Default|GetselectedMini))
  (:Pressed
    (if (Utilities|IsValid _selectedmini)
      (CallFunction|MiniToggleProne _selectedmini))))

(event Input|ActionEvents|InputActionDeleteMini
  (params (Key :type Key%20Structure :default "AnyKey"))
  (bind _selectedmini (Variables|Default|GetselectedMini))
  (:Pressed
    (if (Utilities|IsValid _selectedmini)
      (Actor|DestroyActor _selectedmini))))

(event Input|ActionEvents|InputActionToggleStunned
  (params (Key :type Key%20Structure :default "AnyKey"))
  (bind _selectedmini (Variables|Default|GetselectedMini))
  (:Pressed
    (if (Utilities|IsValid _selectedmini)
      (CallFunction|MiniToggleStunned _selectedmini))))

(event Input|ActionEvents|InputActionQuicksave
  (params (Key :type Key%20Structure :default "AnyKey"))
  (:Pressed
    (Class|FileInteraction|FileSaveString "" "quicksave.txt")))

(event Input|ActionEvents|InputActionQuickload
  (params (Key :type Key%20Structure :default "AnyKey")))

(event Input|ActionEvents|InputActionSpawnMiniA
  (params (Key :type Key%20Structure :default "AnyKey"))
  (:Pressed
    (bind _returnvalue (Game|SpawnActorfromClass "/Game/Blueprints/mini.mini_C" (Math|Transform|MakeTransform "0, 0, 0") "AlwaysSpawn" 0 0))
    (Variables|/Game/Blueprints/mini.mini_C|Setteam _returnvalue 0)
    (Variables|/Game/Blueprints/mini.mini_C|SetteamMaterial _returnvalue "/Game/Material/blue.blue")
    (Variables|/Game/Blueprints/mini.mini_C|SetdoneMaterial _returnvalue "/Game/Material/Blue_done.Blue_done")))

(event Input|ActionEvents|InputActionSpawnMiniB
  (params (Key :type Key%20Structure :default "AnyKey"))
  (:Pressed
    (bind _returnvalue (Game|SpawnActorfromClass "/Game/Blueprints/mini.mini_C" (Math|Transform|MakeTransform "0, 0, 0") "AlwaysSpawn" 0 0))
    (Variables|/Game/Blueprints/mini.mini_C|Setteam _returnvalue 1)
    (Variables|/Game/Blueprints/mini.mini_C|SetteamMaterial _returnvalue "/Game/Material/blue.blue")
    (Variables|/Game/Blueprints/mini.mini_C|SetdoneMaterial _returnvalue "/Game/Material/Blue_done.Blue_done")))

(event Input|ActionEvents|InputActionSpawnBall
  (params (Key :type Key%20Structure :default "AnyKey"))
  (:Pressed
    (bind _returnvalue (Game|SpawnActorfromClass "/Game/Blueprints/mini.mini_C" (Math|Transform|MakeTransform "0, 0, 0") "AlwaysSpawn" 0 0))
    (Variables|/Game/Blueprints/mini.mini_C|Setteam _returnvalue 0)
    (Variables|/Game/Blueprints/mini.mini_C|SetteamMaterial _returnvalue "/Game/Material/metallicBlack.metallicBlack")
    (Variables|/Game/Blueprints/mini.mini_C|SetdoneMaterial _returnvalue "/Game/Material/metallicBlack.metallicBlack")
    (Variables|/Game/Blueprints/mini.mini_C|Setposition _returnvalue "Ball")
    (CallFunction|UpdateMiniRenderers _returnvalue)))

(event Input|ActionEvents|InputActionShowMiniEdit
  (params (Key :type Key%20Structure :default "AnyKey"))
  (:Pressed
    (Default|ToggleMiniEdit (Variables|Default|GethudRef))))

(event Input|ActionEvents|InputActionToggleDone
  (params (Key :type Key%20Structure :default "AnyKey"))
  (bind _selectedmini (Variables|Default|GetselectedMini))
  (:Pressed
    (if (Utilities|IsValid _selectedmini)
      (CallFunction|MiniToggleDone _selectedmini))))

(event Input|MouseEvents|LeftMouseButton
  (params (Key :type Key%20Structure :default "AnyKey"))
  (bind _array (Utilities|Array|MakeArray "ObjectTypeQuery2"))
  (bind (_hitresult _returnvalue) (Class|PlayerController|GetHitResultUnderCursorforObjects _array true))
  (:Pressed
    (Variables|Default|Setclicking true)
    (if _returnvalue
      (Utilities|FlowControl|Sequence
        (:then_0
          (if (Utilities|IsValid (Variables|Default|GetselectedMini)) :!label _label
            (Default|SetSelected (Variables|Default|GetselectedMini) false))
          (Variables|Default|SetselectedMini 0)
          (Default|ClearMiniText (Variables|Default|GethudRef)))
        (:then_1
          (bind _asmini (Utilities|Casting|CastTomini (.HitActor (Collision|BreakHitResult _hitresult))))
          (bind _output_get (Variables|Default|SetselectedMini _asmini))
          (Default|SetSelected _output_get true)
          (Default|UpdateMiniText (Variables|Default|GethudRef))))
      (else
        (goto _label))))
  (:Released
    (Variables|Default|Setclicking false)
    (if (Utilities|IsValid (Variables|Default|GetselectedMini))
      (CallFunction|SnapMinitoGrid (Variables|Default|GetselectedMini)))))

(fn ConstructionScript)

(fn PingatMouseCursor)

(fn GetSaveString
  (bind _outactors (Actor|GetAllActorsOfClass "/Game/Blueprints/mini.mini_C"))
  (for _array_element _outactors
    _))

(fn InitializeGame
  (bind (_savetexta _returnvalue) (Class|FileInteraction|FileLoadString "init.txt"))
  (if _returnvalue
    (LocalVariables|Settmp _savetexta)
    (while (LocalVariables|Getcontinue)
      (if (.ReturnValue (Utilities|String|Split (LocalVariables|Gettmp) "\\n"))
        (LocalVariables|Settmp (.RightS (Utilities|String|Split (LocalVariables|Gettmp) "\\n")))))
    (else
      (return false))))