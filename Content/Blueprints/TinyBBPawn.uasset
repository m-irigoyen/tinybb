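; TinyBBPawn is a pawn that pans and zooms from player axis input, apparently as a top-down camera.
; Up and Right inputs offset its location along the negated right vector and the forward vector, scaled by MoveSpeed without delta time or sweeping.
; Zoom input adjusts a clamped target height, initialised from the actor's Z in the construction script.
; Tick interpolates the actor's height toward that target for smooth zooming.
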(event EventTick
  (params (DeltaSeconds :type Float%20%28single-precision%29))
  (bind _returnvalue (Transformation|GetActorLocation))
  (bind (_x _y) (Math|Vector|BreakVector _returnvalue))
  (Transformation|SetActorLocation (Math|Interpolation|VInterpTo _returnvalue (Math|Vector|MakeVector _x _y (Variables|Default|GetdesiredZ)) DeltaSeconds (Variables|Default|GetzoomInterpSpeed)) false false))

(event Input|AxisEvents|InputAxisUp
  (params (AxisValue :type Float%20%28single-precision%29))
  (Transformation|SetActorLocation (+ (Transformation|GetActorLocation) (* (* (Transformation|GetActorRightVector) -1.0) (* AxisValue (Variables|Default|GetmoveSpeed)))) false false))

(event Input|AxisEvents|InputAxisRight
  (params (AxisValue :type Float%20%28single-precision%29))
  (Transformation|SetActorLocation (+ (Transformation|GetActorLocation) (* (Transformation|GetActorForwardVector) (* AxisValue (Variables|Default|GetmoveSpeed)))) false false))

(event Input|AxisEvents|InputAxisZoom
  (params (AxisValue :type Float%20%28single-precision%29))
  (Variables|Default|SetdesiredZ (Math|Float|Clamp(Float) (+ (Variables|Default|GetdesiredZ) (* AxisValue (Variables|Default|GetzoomTick))) (Variables|Default|GetmaxZoom) (Variables|Default|GetminZoom))))

(fn ConstructionScript
  (Variables|Default|SetdesiredZ (.Z (Math|Vector|BreakVector (Transformation|GetActorLocation)))))