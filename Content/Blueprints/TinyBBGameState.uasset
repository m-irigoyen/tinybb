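; Game state Blueprint for TinyBB that holds score, turn and RR counters for two teams, A and B.
; ChangeScore, ChangeTurn and ChangeRR each take a team flag and an Adding flag, then step that team's counter up or down by one.
; The counters have no bounds checks, and the event graph and construction script contain no active logic.
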(event EventBeginPlay)

(event EventTick
  (params (DeltaSeconds :type Float%20%28single-precision%29)))

(fn ConstructionScript)

(fn ChangeScore
  (params (teamA :type Boolean) (adding :type Boolean))
  (if adding
    (LocalVariables|Settmp 1)
    (else
      (LocalVariables|Settmp -1)))
  (if teamA
    (Variables|Default|SetAScore (+ (Variables|Default|GetAScore) (LocalVariables|Gettmp)))
    (else
      (Variables|Default|SetBScore (+ (Variables|Default|GetBScore) (LocalVariables|Gettmp))))))

(fn ChangeTurn
  (params (teamA :type Boolean) (adding :type Boolean))
  (if adding
    (LocalVariables|Settmp 1)
    (else
      (LocalVariables|Settmp -1)))
  (if teamA
    (Variables|Default|SetATurn (+ (Variables|Default|GetATurn) (LocalVariables|Gettmp)))
    (else
      (Variables|Default|SetBTurn (+ (Variables|Default|GetBTurn) (LocalVariables|Gettmp))))))

(fn ChangeRR
  (params (teamA :type Boolean) (adding :type Boolean))
  (if adding
    (LocalVariables|Settmp 1)
    (else
      (LocalVariables|Settmp -1)))
  (if teamA
    (Variables|Default|SetARR (+ (Variables|Default|GetARR) (LocalVariables|Gettmp)))
    (else
      (Variables|Default|SetBRR (+ (Variables|Default|GetBRR) (LocalVariables|Gettmp))))))