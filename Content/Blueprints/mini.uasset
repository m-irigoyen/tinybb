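; Player miniature actor for a grid-based, ball-carrying team game, showing position text, number, team material and status markers.
; The construction script applies labels and material and hides all markers; setters and toggles drive ball, prone, stunned and done state, with done swapping the sphere material.
; Stunning a standing piece first makes it prone, while setting prone clears an existing stun.
; SnapToGrid centres the actor in its grid cell at zero height.
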(event EventBeginPlay)

(event Collision|EventActorBeginOverlap
  (params (OtherActor :type Actor%20Object%20Reference)))

(event EventTick
  (params (DeltaSeconds :type Float%20%28single-precision%29)))

(fn ConstructionScript
  (CallFunction|UpdateRenderers)
  (Rendering|SetVisibility (Variables|Default|Getball) false false)
  (Rendering|SetVisibility (Variables|Default|GetcrossProne) false false)
  (Rendering|SetVisibility (Variables|Default|GetselectedCircle) false false)
  (Rendering|SetVisibility (Variables|Default|GetcrossStun) false false))

(fn UpdateRenderers
  (Rendering|Components|TextRender|SetText (Variables|Default|GetNameText) (Variables|Default|Getposition))
  (Rendering|Components|TextRender|SetText (Variables|Default|GetNumberText) (Utilities|Text|ToText(Integer) (Variables|Default|Getnumber)))
  (Rendering|Material|SetMaterial (Variables|Default|GetSphere) 0 (Variables|Default|GetteamMaterial)))

(fn SnaptoGrid
  (bind _returnvalue (Transformation|GetActorLocation))
  (bind (_x _y) (Math|Vector|BreakVector _returnvalue))
  (if true
    (Transformation|SetActorLocation (Math|Vector|MakeVector (+ (* (Math|Conversions|ToFloat(Integer) (Math|Float|Floor (/ _x 1e+02))) 1e+02) 5e+01) (+ (* (Math|Conversions|ToFloat(Integer) (Math|Float|Floor (/ _y 1e+02))) 1e+02) 5e+01) 0.0) false false)))

(fn ToggleBall
  (CallFunction|SetBall (not (Variables|Default|GethasBall))))

(fn ToggleDone
  (CallFunction|SetDone (not (Variables|Default|GetisDone))))

(fn SetSelected
  (params (selected :type Boolean))
  (Rendering|SetVisibility (Variables|Default|GetselectedCircle) selected true))

(fn ToggleProne
  (CallFunction|SetProne (not (Variables|Default|GetisProne))))

(fn ToggleStunned
  (CallFunction|SetStunned (not (Variables|Default|GetisStunned))))

(fn SetProne
  (params (prone :type Boolean))
  (bind _output_get (Variables|Default|SetisProne prone))
  (Rendering|SetVisibility (Variables|Default|GetcrossProne) _output_get false)
  (if (and (Variables|Default|GetisProne) (Variables|Default|GetisStunned))
    (CallFunction|SetStunned false)))

(fn SetStunned
  (params (stunned :type Boolean))
  (if (and stunned (not (Variables|Default|GetisProne)))
    (CallFunction|SetProne true))
  (bind _output_get (Variables|Default|SetisStunned stunned))
  (Rendering|SetVisibility (Variables|Default|GetcrossStun) _output_get false))

(fn SetBall
  (params (hasBall :type Boolean))
  (bind _output_get (Variables|Default|SethasBall hasBall))
  (Rendering|SetVisibility (Variables|Default|Getball) _output_get false))

(fn SetDone
  (params (done :type Boolean))
  (bind _output_get (Variables|Default|SetisDone done))
  (if _output_get
    (Rendering|Material|SetMaterial (Variables|Default|GetSphere) 0 (Variables|Default|GetdoneMaterial))
    (else
      (Rendering|Material|SetMaterial (Variables|Default|GetSphere) 0 (Variables|Default|GetteamMaterial)))))